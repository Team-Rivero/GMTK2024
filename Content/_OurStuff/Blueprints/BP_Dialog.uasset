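; BP_Dialog is a placeable trigger that shows a configured dialog line through the hamster's UI when overlapped.
; The construction script uses BoxSphere to pick the box or sphere volume, toggling visibility and overlap events.
; The sphere fires once unless Looping is set, while the box bypasses that check and always goes through the shared DoOnce.
; Text and duration are configurable, but the expression passed is fixed, leaving the Expression variable unused.
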(event `self.Sphere.OnComponentBeginOverlap`
  (params (OverlappedComponent :type "PrimitiveComponent Object Reference") (OtherActor :type "Actor Object Reference") (OtherComp :type "PrimitiveComponent Object Reference") (OtherBodyIndex :type Integer) (bFromSweep :type Boolean) (SweepResult :type "HitResult Structure (by ref)"))
  (if (not (`self.Looping?`))
    (`/Engine/EditorBlueprintResources/StandardMacros.DoOnce` false :!label _label
      (:`Completed`
        _)))
  (`/Game/_OurStuff/Widgets/W_UI.Dialog` (`/Game/_OurStuff/Blueprints/FirstPerson/Blueprints/BP_Hamster.UI` (`/Game/_OurStuff/Blueprints/BPM_Actor.GetMyHamster`)) (`self.Text`) (`self.Duration Seconds`) "NewEnumerator0"))

(event `self.Box.OnComponentBeginOverlap`
  (params (OverlappedComponent :type "PrimitiveComponent Object Reference") (OtherActor :type "Actor Object Reference") (OtherComp :type "PrimitiveComponent Object Reference") (OtherBodyIndex :type Integer) (bFromSweep :type Boolean) (SweepResult :type "HitResult Structure (by ref)"))
  (goto _label))

(fn `UserConstructionScript`
  (bind _box (`self.Box`))
  (bind _sphere (`self.Sphere`))
  (bind _box_sphere (`self.Box/Sphere`))
  (bind _returnvalue (not (`self.Box/Sphere`)))
  (`SceneComponent.SetVisibility` _box _box_sphere false)
  (set `PrimitiveComponent.bGenerateOverlapEvents` _box_sphere _box)
  (`SceneComponent.SetVisibility` _sphere _returnvalue false)
  (set `PrimitiveComponent.bGenerateOverlapEvents` _returnvalue _sphere))