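; BP_Static_Scaling is an actor that smoothly shrinks or grows when it receives the Shrink/Grow interface event.
; The event multiplies a stored target scale, seeded from the root's X scale at BeginPlay, and turns on Tick.
; Tick eases the root's world scale toward the target at a rate proportional to current scale, remaining difference and a speed modifier, then disables itself once nearly there.
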(event `self.ReceiveBeginPlay`
  (bind _returnvalue_x (`KismetMathLibrary.BreakVector` (`SceneComponent.K2_GetComponentScale` (`self.DefaultSceneRoot`))))
  ;[1 1 1] Begin Play
  (set `self.NewScale` _returnvalue_x))

(event `self.ReceiveTick`
  (params (DeltaSeconds :type "Float (single-precision)"))
  (bind _defaultsceneroot (`self.DefaultSceneRoot`))
  (bind _returnvalue_x (`KismetMathLibrary.BreakVector` (`SceneComponent.K2_GetComponentScale` (`self.DefaultSceneRoot`))))
  (bind _returnvalue (- (`self.NewScale`) _returnvalue_x))
  (bind _returnvalue_2 (* DeltaSeconds _returnvalue_x _returnvalue (`self.ScaleSpeedModifier`)))
  ;[1 0.3694 0.3097] Tick
  (if (> (`KismetMathLibrary.Abs` _returnvalue) 0.001)
    (`SceneComponent.SetWorldScale3D` _defaultsceneroot (+ (`SceneComponent.K2_GetComponentScale` _defaultsceneroot) (`KismetMathLibrary.MakeVector` _returnvalue_2 _returnvalue_2 _returnvalue_2)))
    (else
      (`self.SetActorTickEnabled` false))))

(event `self.Shrink/Grow`
  (params (`Shrink/Grow Scalar` :type "Float (double-precision)"))
  ;[1 1 1] BPI Shrink/Grow
  (set `self.NewScale` (* `Shrink/Grow Scalar` (`self.NewScale`)))
  (`self.SetActorTickEnabled` true))

(fn `UserConstructionScript`)