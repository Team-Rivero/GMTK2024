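; Actor that smoothly grows or shrinks when it receives the BPI Shrink/Grow interface event.
; Each event multiplies the target scale, initialized from the root's world X scale, and enables Tick.
; Tick adds equal steps to all axes, proportional to current X scale, remaining difference and ScaleSpeedModifier, and prints debug values.
; Tick disables itself once X is within a small tolerance of the target.
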(event `self.ReceiveBeginPlay`
  (bind _returnvalue_x (`KismetMathLibrary.BreakVector` (`SceneComponent.K2_GetComponentScale` (`self.DefaultSceneRoot`))))
  ;[1 1 1] Begin Play
  (set `self.New Scale` _returnvalue_x))

(event `self.ReceiveTick`
  (params (DeltaSeconds :type "Float (single-precision)"))
  (bind _defaultsceneroot (`self.DefaultSceneRoot`))
  (bind _returnvalue_x (`KismetMathLibrary.BreakVector` (`SceneComponent.K2_GetComponentScale` _defaultsceneroot)))
  (bind _returnvalue (- (`self.New Scale`) _returnvalue_x))
  (bind _returnvalue_2 (* DeltaSeconds _returnvalue_x _returnvalue (`self.Scale Speed Modifier`)))
  (bind _returnvalue_3 (+ (`SceneComponent.K2_GetComponentScale` _defaultsceneroot) (`KismetMathLibrary.MakeVector` _returnvalue_2 _returnvalue_2 _returnvalue_2)))
  ;[1 0.3694 0.3097] Tick
  (if (> (`KismetMathLibrary.Abs` _returnvalue) 0.001)
    (`SceneComponent.SetWorldScale3D` _defaultsceneroot _returnvalue_3)
    (`KismetSystemLibrary.PrintString` (`KismetStringLibrary.Conv_VectorToString` _returnvalue_3))
    (else
      (`self.SetActorTickEnabled` false))))

(event `/Game/_OurStuff/Blueprints/BPI_ShrinkGrow.Shrink/Grow`
  (params (`Shrink/Grow Scalar` :type "Float (double-precision)"))
  ;[1 1 1] BPI Shrink/Grow
  (set `self.New Scale` (* `Shrink/Grow Scalar` (`self.New Scale`)))
  (`self.SetActorTickEnabled` true))

(fn `UserConstructionScript`)