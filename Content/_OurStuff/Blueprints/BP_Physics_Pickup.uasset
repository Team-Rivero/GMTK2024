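; Physics pickup actor that the hamster player can grab and drop.
; When free, Tick uses distance and a view-direction dot product to register it in the hamster's InteractingActors and toggle its prompt widget.
; Interact toggles holding, switching gravity, zeroing velocities and updating the hamster's held-object buffer.
; While held, the cube follows the hamster's hold point and arrow rotation each tick with a swept move.
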(event `self.ReceiveTick`
  (params (DeltaSeconds :type "Float (single-precision)"))
  (bind _asbp_hampster (`/Game/_OurStuff/Blueprints/BPM_Actor.GetMyHamster`))
  (bind _asbp_hampster_2 (`/Game/_OurStuff/Blueprints/BPM_Actor.GetMyHamster`))
  (bind _asbp_hampster_3 (`/Game/_OurStuff/Blueprints/BPM_Actor.GetMyHamster`))
  (bind _widget (`self.Widget`))
  (bind _interactingactors (`/Game/_OurStuff/Blueprints/FirstPerson/Blueprints/BP_Hamster.InteractingActors` _asbp_hampster_2))
  (bind _returnvalue (`KismetArrayLibrary.Array_Contains` (`/Game/_OurStuff/Blueprints/FirstPerson/Blueprints/BP_Hamster.InteractingActors` _asbp_hampster_2) self))
  (bind _returnvalue_2 (- (`SceneComponent.K2_GetComponentLocation` (`self.Cube`)) (`self.K2_GetActorLocation` _asbp_hampster_3)))
  ;[1 0.276 0.276] Tick
  (if (`self.Held`)
    (`SceneComponent.K2_SetWorldLocationAndRotation` (`self.Cube`) (`SceneComponent.K2_GetComponentLocation` (`/Game/_OurStuff/Blueprints/FirstPerson/Blueprints/BP_Hamster.Held Object` _asbp_hampster)) (`SceneComponent.K2_GetComponentRotation` (`/Game/_OurStuff/Blueprints/FirstPerson/Blueprints/BP_Hamster.Arrow1` _asbp_hampster)) true false)
    (elif (and (< (`KismetMathLibrary.VSize` _returnvalue_2) (`self.Pickup Distance`)) (> (`KismetMathLibrary.Dot_VectorVector` (`KismetMathLibrary.Normal` _returnvalue_2) (`KismetMathLibrary.GetForwardVector` (`Pawn.GetControlRotation` _asbp_hampster_3))) (`self.Pickup Tolerance`)))
      (if (not _returnvalue)
        (`KismetArrayLibrary.Array_AddUnique` _interactingactors self)
        (`SceneComponent.SetHiddenInGame` _widget false false))
      (elif _returnvalue
        (`KismetArrayLibrary.Array_RemoveItem` _interactingactors self)
        (`SceneComponent.SetHiddenInGame` _widget true false)))))

(event `/Game/_OurStuff/Blueprints/BPI_Interact.Interact`
  (bind _asbp_hampster (`/Game/_OurStuff/Blueprints/BPM_Actor.GetMyHamster`))
  (bind _cube (`self.Cube`))
  (bind _heldobject (`/Game/_OurStuff/Blueprints/FirstPerson/Blueprints/BP_Hamster.HeldObject` (`/Game/_OurStuff/Blueprints/BPM_Actor.GetMyHamster`)))
  ;[1 1 1] Interact
  (if (and _heldobject (`self.Held`))
    (set `/Game/_OurStuff/Blueprints/FirstPerson/Blueprints/BP_Hamster.HeldObjectBuffer` false _asbp_hampster)
    (set `self.Held` false)
    (`PrimitiveComponent.SetEnableGravity` _cube true)
    (`PrimitiveComponent.SetPhysicsLinearVelocity` _cube (0.0 0.0 0.0) false "None" :!label _label)
    (`PrimitiveComponent.SetPhysicsAngularVelocityInDegrees` _cube (0.0 0.0 0.0) false "None")
    (elif (not _heldobject)
      (set `self.Held` true)
      (set `/Game/_OurStuff/Blueprints/FirstPerson/Blueprints/BP_Hamster.HeldObjectBuffer` true _asbp_hampster)
      (`PrimitiveComponent.SetEnableGravity` _cube false)
      (goto _label))))

(fn `UserConstructionScript`)