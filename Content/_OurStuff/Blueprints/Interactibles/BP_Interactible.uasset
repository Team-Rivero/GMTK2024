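; BP_Interactible is a world object that the player's hamster can interact with, consuming it with a chomp sound.
; Overlapping its sphere collision adds it to the hamster's InteractingActors list and shows its widget; ending the overlap removes it and hides the widget.
; The Interact event destroys the actor and plays the Chomp sound in 2D.
; The overlap handlers do not check which actor triggered them.
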(event `/Game/_OurStuff/Blueprints/BPI_Interact.Interact`
  (`self.K2_DestroyActor`)
  (`GameplayStatics.PlaySound2D` "/Game/_OurStuff/Audio/chomp.chomp" 0.5 1.0 0.0 null null))

(event `self.SphereCollision.OnComponentBeginOverlap`
  (params (OverlappedComponent :type "PrimitiveComponent Object Reference") (OtherActor :type "Actor Object Reference") (OtherComp :type "PrimitiveComponent Object Reference") (OtherBodyIndex :type Integer) (bFromSweep :type Boolean) (SweepResult :type "HitResult Structure (by ref)"))
  (`KismetArrayLibrary.Array_AddUnique` (`/Game/_OurStuff/Blueprints/FirstPerson/Blueprints/BP_Hamster.InteractingActors` (`/Game/_OurStuff/Blueprints/BPM_Actor.GetMyHamster`)) self)
  (`SceneComponent.SetHiddenInGame` (`self.Widget`) false false))

(event `self.SphereCollision.OnComponentEndOverlap`
  (params (OverlappedComponent :type "PrimitiveComponent Object Reference") (OtherActor :type "Actor Object Reference") (OtherComp :type "PrimitiveComponent Object Reference") (OtherBodyIndex :type Integer))
  (`KismetArrayLibrary.Array_RemoveItem` (`/Game/_OurStuff/Blueprints/FirstPerson/Blueprints/BP_Hamster.InteractingActors` (`/Game/_OurStuff/Blueprints/BPM_Actor.GetMyHamster`)) self)
  (`SceneComponent.SetHiddenInGame` (`self.Widget`) true false))

(fn `UserConstructionScript`)