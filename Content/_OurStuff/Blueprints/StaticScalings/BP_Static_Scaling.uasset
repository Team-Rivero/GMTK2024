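; Actor that shrinks or grows uniformly when it receives a Shrink/Grow event with a multiplier.
; The multiplier compounds into a target scale, and a timeline lerps toward it, applying only values between the shrink and growth limits.
; On finish, the target resyncs to the actual scale.
; An older tick- and curve-based scaler with reverse-on-overlap remains in the graph but is disconnected, leaving ReverseScale inactive.
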(event `self.ReceiveActorBeginOverlap`
  (params (OtherActor :type "Actor Object Reference"))
  ;[1 1 1] stop on overlap
)

(event `Unlock Reversing`
  ;[1 1 1] stop on overlap
  (`/Engine/EditorBlueprintResources/StandardMacros.DoOnce` false :!via `Reset`
    (:`Completed`
      (`self.ReverseScale`))))

(event `self.ReceiveBeginPlay`
  ;[1 1 1] Begin Play
)

(event `self.ReceiveTick`
  (params (DeltaSeconds :type "Float (single-precision)"))
  ;[1 0.3694 0.3097] Tick
)

(event `/Game/_OurStuff/Blueprints/BPI_ShrinkGrow.Shrink/Grow`
  (params (`Shrink/Grow Scalar` :type "Float (double-precision)"))
  (bind _returnvalue_x (`KismetMathLibrary.BreakVector` (`SceneComponent.K2_GetComponentScale` (`self.DefaultSceneRoot`))))
  (bind _returnvalue_x_2 (`KismetMathLibrary.BreakVector` (`SceneComponent.K2_GetComponentScale` (`self.DefaultSceneRoot`))))
  (set `self.CurrentScale` _returnvalue_x)
  (set `self.NewScale` (* `Shrink/Grow Scalar` (`self.NewScale`)))
  (bind (_direction _alpha) (`Timeline|Scale` :!via `PlayFromStart`)
    (:`Update`
      (bind _returnvalue (`KismetMathLibrary.Lerp` (`self.CurrentScale`) (`self.NewScale`) _alpha))
      (if (and (< (`self.ShrinkLimit`) _returnvalue) (> (`self.GrowthLimit`) _returnvalue))
        (`SceneComponent.SetWorldScale3D` (`self.DefaultSceneRoot`) (`KismetMathLibrary.Conv_DoubleToVector` _returnvalue))))
    (:`Finished`
      (set `self.NewScale` _returnvalue_x_2))))

(fn `ReverseScale`
  (locals (TempScale :type "Float (double-precision)"))
  (set `local.TempScale` (`self.NewScale`))
  (set `self.NewScale` (`self.PreviousScale`))
  (set `self.PreviousScale` (`local.TempScale`))
  (set `self.ScaleTimeRemaining` (- (`self.ScaleDuration`) (`self.ScaleTimeRemaining`)))
  (`self.SetActorTickEnabled` true))

(fn `UserConstructionScript`)