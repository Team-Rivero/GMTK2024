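; Activatable door that swings on a hinge: any activation opens it, but only a non-user activation can close it again.
; Activate toggles the open state and plays a timeline forward or in reverse, turning the hinge by per-update yaw deltas toward a configurable angle.
; A widget hides during motion, then moves to the door mesh's location when finished, showing only if the door is closed.
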(event `/Game/_OurStuff/Blueprints/BPI_Activate.Activate`
  (params (UserActivated :type Boolean))
  (if (`self.Open`)
    (if (not UserActivated)
      (`SceneComponent.SetVisibility` (`self.Widget`) false false :!label _label)
      (set `self.Open` (not (`self.Open`)))
      (if (`self.Open`)
        (set `self.CurrentAngle` 0.0)
        (bind (_direction _opening) (`Timeline|Timeline` :!via `PlayFromStart` :!label _label_2)
          (:`Update`
            (bind _returnvalue (`KismetMathLibrary.Lerp` 0.0 (`self.HingeAngle`) _opening))
            (bind _returnvalue_2 (- (`self.CurrentAngle`) _returnvalue))
            (`SceneComponent.K2_AddLocalRotation` (`self.Hinge`) (`KismetMathLibrary.MakeRotator` 0.0 0.0 _returnvalue_2) false false)
            (set `self.CurrentAngle` _returnvalue))
          (:`Finished`
            (`SceneComponent.SetVisibility` (`self.Widget`) (not (`self.Open`)) false)
            (`SceneComponent.K2_AddLocalRotation` (`self.Hinge`) (`KismetMathLibrary.MakeRotator` 0.0 0.0 _returnvalue_2) false false)
            (set `self.CurrentAngle` _returnvalue)
            (`SceneComponent.K2_SetWorldLocation` (`self.Widget`) (`SceneComponent.K2_GetComponentLocation` (`self.DoorMesh`)) false false)))
        (else
          (set `self.CurrentAngle` (`self.HingeAngle`))
          (goto _label_2 :!via `ReverseFromEnd`))))
    (else
      (goto _label))))

(fn `UserConstructionScript`
  (`parent.UserConstructionScript`))