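; BP_Button is a pressure button that activates a linked ActivatableActor when a weighable actor rests on it.
; Overlap stores any BPI_Weighable actor and fires immediately if SizeRequirement is zero.
; Tick also fires through a DoOnce, never reset here, while that actor overlaps with X scale meeting the requirement.
; A timeline sinks the button mesh on activation, and ReleaseButton reverses it without deactivating the target.
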(event `self.Collision.OnComponentBeginOverlap`
  (params (OverlappedComponent :type "PrimitiveComponent Object Reference") (OtherActor :type "Actor Object Reference") (OtherComp :type "PrimitiveComponent Object Reference") (OtherBodyIndex :type Integer) (bFromSweep :type Boolean) (SweepResult :type "HitResult Structure (by ref)"))
  (bind _activatableactor (`self.ActivatableActor`))
  (if (`KismetSystemLibrary.DoesImplementInterface` OtherActor "/Game/_OurStuff/Blueprints/BPI_Weighable.BPI_Weighable_C")
    (set `self.Other Actor` OtherActor)
    (if (== (`self.SizeRequirement`) 0.0)
      (`/Engine/EditorBlueprintResources/StandardMacros.IsValid` _activatableactor :!label _label
        (:`Is Valid`
          (`/Game/_OurStuff/Blueprints/BPI_Activate.Activate` _activatableactor true)
          (bind (_direction _newtrack_0) (`Timeline|Timeline` :!via `PlayFromStart` :!label _label_2)
            (:`Update`
              (`SceneComponent.K2_SetWorldLocation` (`self.button`) (- (`SceneComponent.K2_GetComponentLocation` (`self.DefaultSceneRoot`)) (`KismetMathLibrary.MakeVector` 0.0 0.0 (* _newtrack_0 4.0))) false true))))))))

(event `Release Button`
  (goto _label_2 :!via `Reverse`))

(event `self.ReceiveTick`
  (params (DeltaSeconds :type "Float (single-precision)"))
  (bind _other_actor (`self.Other Actor`))
  (bind _returnvalue_x (`KismetMathLibrary.BreakVector` (`self.GetActorScale3D` _other_actor)))
  (`/Engine/EditorBlueprintResources/StandardMacros.IsValid` _other_actor
    (:`Is Valid`
      (if (and (`PrimitiveComponent.IsOverlappingActor` (`self.Collision`) _other_actor) (>= _returnvalue_x (`self.SizeRequirement`)))
        (`/Engine/EditorBlueprintResources/StandardMacros.DoOnce` false
          (:`Completed`
            (goto _label)))))))

(fn `UserConstructionScript`)