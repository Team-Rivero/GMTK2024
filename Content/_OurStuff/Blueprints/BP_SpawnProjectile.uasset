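; BP_SpawnProjectile is a timed spawner that fires BP_RayProjectile actors from its own location, alternating between grow and shrink variants.
; After a short delay on BeginPlay, it spawns the first projectile, then a self-calling Loop event with a Delay repeats the spawn indefinitely.
; Each loop flips the GrowShrink flag, which is passed to the projectile along with a matching scale-up or scale-down scalar.
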(event `Loop`
  (bind _grow__shrink (`self.Grow/ Shrink`))
  (set `self.Grow/ Shrink` (not (`self.Grow/ Shrink`)))
  (`|SpawnActorFromClass` "/Game/_OurStuff/Blueprints/FirstPerson/Blueprints/BP_RayProjectile.BP_RayProjectile_C" (`KismetMathLibrary.MakeTransform` (`self.K2_GetActorLocation`)) "Undefined" "OverrideRootScale" null (`KismetMathLibrary.SelectFloat` 1.5 0.66 _grow__shrink) _grow__shrink null :!label _label)
  (`KismetSystemLibrary.Delay` 2.0)
  (`self.Loop`))

(event `self.ReceiveBeginPlay`
  (`KismetSystemLibrary.Delay` 1.0)
  (goto _label))

(fn `UserConstructionScript`)