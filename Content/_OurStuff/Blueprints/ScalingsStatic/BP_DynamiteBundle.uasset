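; A scalable dynamite bundle actor that reacts to the parent class's Shrink/Grow event.
; Above a world scale of 2, it registers in the hamster's InteractingActors and shows its widget; otherwise it unregisters and hides it.
; Interact is a stub: the explode-and-destroy logic for scales between 2 and 6 is disconnected and never runs, and a UI Sticks check is left unused.
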(event `/Game/_OurStuff/Blueprints/BPI_ShrinkGrow.Shrink/Grow`
  (params (`Shrink/Grow Scalar` :type "Float (double-precision)"))
  (bind _widget (`self.Widget`))
  (bind _returnvalue_x (`KismetMathLibrary.BreakVector` (`SceneComponent.K2_GetComponentScale` (`self.DefaultSceneRoot`))))
  (bind _interactingactors (`/Game/_OurStuff/Blueprints/FirstPerson/Blueprints/BP_Hamster.InteractingActors` (`/Game/_OurStuff/Blueprints/BPM_Actor.GetMyHamster`)))
  (`parent.Shrink/Grow` `Shrink/Grow Scalar`)
  (if (> _returnvalue_x 2.0)
    (`KismetArrayLibrary.Array_AddUnique` _interactingactors self)
    (`SceneComponent.SetHiddenInGame` _widget false false)
    (else
      (`KismetArrayLibrary.Array_RemoveItem` _interactingactors self)
      (`SceneComponent.SetHiddenInGame` _widget true false))))

(event `/Game/_OurStuff/Blueprints/BPI_Interact.Interact`
  (if true
    _))

(fn `UserConstructionScript`
  (`parent.UserConstructionScript`))