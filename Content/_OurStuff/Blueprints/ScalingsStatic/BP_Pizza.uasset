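; BP_Pizza is an interactable pizza that the player's hamster eats piece by piece over five bites.
; Sphere overlap registers it in the hamster's InteractingActors and toggles a prompt widget.
; Each interaction removes one static mesh piece, plays a chomp and shows hamster UI dialog, destroying the actor after the last.
; The pizza's world scale sets both the chomp pitch, lower when bigger, and the dialog line.
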(event `self.ReceiveBeginPlay`
  (`parent.ReceiveBeginPlay`)
  (set `self.Array` (`|MakeArray` (`self.StaticMesh5`) (`self.StaticMesh1`) (`self.StaticMesh2`) (`self.StaticMesh3`) (`self.StaticMesh4`))))

(event `self.Sphere.OnComponentBeginOverlap`
  (params (OverlappedComponent :type "PrimitiveComponent Object Reference") (OtherActor :type "Actor Object Reference") (OtherComp :type "PrimitiveComponent Object Reference") (OtherBodyIndex :type Integer) (bFromSweep :type Boolean) (SweepResult :type "HitResult Structure (by ref)"))
  (if (< (`self.NewVar_1`) 5)
    (`KismetArrayLibrary.Array_AddUnique` (`/Game/_OurStuff/Blueprints/FirstPerson/Blueprints/BP_Hamster.InteractingActors` (`/Game/_OurStuff/Blueprints/BPM_Actor.GetMyHamster`)) self)
    (`SceneComponent.SetHiddenInGame` (`self.Widget`) false false)))

(event `self.Sphere.OnComponentEndOverlap`
  (params (OverlappedComponent :type "PrimitiveComponent Object Reference") (OtherActor :type "Actor Object Reference") (OtherComp :type "PrimitiveComponent Object Reference") (OtherBodyIndex :type Integer))
  (`KismetArrayLibrary.Array_RemoveItem` (`/Game/_OurStuff/Blueprints/FirstPerson/Blueprints/BP_Hamster.InteractingActors` (`/Game/_OurStuff/Blueprints/BPM_Actor.GetMyHamster`)) self)
  (`SceneComponent.SetHiddenInGame` (`self.Widget`) true false))

(event `/Game/_OurStuff/Blueprints/BPI_Interact.Interact`
  (bind _returnvalue_x (`KismetMathLibrary.BreakVector` (`SceneComponent.K2_GetComponentScale` (`self.DefaultSceneRoot`))))
  (if (< (`self.NewVar_1`) 5)
    (`GameplayStatics.PlaySound2D` "/Game/_OurStuff/Audio/chomp.chomp" 0.5 (`KismetMathLibrary.MapRangeClamped` _returnvalue_x 2.0 12.0 1.5 0.5) 0.0 null null)
    (`ActorComponent.K2_DestroyComponent` (`|GetArrayItem` (`self.Array`) (`self.NewVar_1`)))
    (`/Game/_OurStuff/Widgets/W_UI.Dialog` (`/Game/_OurStuff/Blueprints/FirstPerson/Blueprints/BP_Hamster.UI` (`/Game/_OurStuff/Blueprints/BPM_Actor.GetMyHamster`)) (`|GetArrayItem` (`self.Text_0`) (select `int` (`KismetMathLibrary.Round` _returnvalue_x) :`0` 0 :`1` 0 :`2` 0 :`3` 1 :`4` 1 :`5` 1 :`6` 2 :`7` 2 :`8` 2 :`9` 2 :`10` 2 :`11` 2 :`12` 3)) 1.5 "NewEnumerator0")
    (`/Engine/EditorBlueprintResources/StandardMacros.IncrementInt` (`self.NewVar_1`)
      (:`  `
        (if (not (< (`self.NewVar_1`) 5))
          (`SceneComponent.SetHiddenInGame` (`self.Widget`) true false)
          (`self.K2_DestroyActor`))))))

(fn `UserConstructionScript`
  (`parent.UserConstructionScript`))