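; Hamster wheel actor that spins up and changes the player hamster's walk speed while its capsule is overlapped.
; Capsule begin and end overlap play and reverse one Timeline, with no check on the overlapping actor.
; The Timeline feeds a roll rate and the hamster's MaxWalkSpeed, easing both in and out.
; Tick applies that roll to the wheel every frame, unscaled by delta time.
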(event `self.ReceiveTick`
  (params (DeltaSeconds :type "Float (single-precision)"))
  (`parent.ReceiveTick` DeltaSeconds)
  (`self.SetActorTickEnabled` true)
  (`SceneComponent.K2_AddLocalRotation` (`self.Wheel`) (`KismetMathLibrary.MakeRotator` (`self.Delta Rotation X (Roll)`)) false false))

(event `self.Capsule.OnComponentBeginOverlap`
  (params (OverlappedComponent :type "PrimitiveComponent Object Reference") (OtherActor :type "Actor Object Reference") (OtherComp :type "PrimitiveComponent Object Reference") (OtherBodyIndex :type Integer) (bFromSweep :type Boolean) (SweepResult :type "HitResult Structure (by ref)"))
  (`self.Play`))

(event `self.Capsule.OnComponentEndOverlap`
  (params (OverlappedComponent :type "PrimitiveComponent Object Reference") (OtherActor :type "Actor Object Reference") (OtherComp :type "PrimitiveComponent Object Reference") (OtherBodyIndex :type Integer))
  (`self.Reverse`))

(event `Play`
  (bind (_direction _rotationspeed _walkspeed) (`Timeline|Timeline` :!label _label)
    (:`Update`
      (set `self.Delta Rotation X (Roll)` _rotationspeed)
      (set `CharacterMovementComponent.MaxWalkSpeed` _walkspeed (`Character.CharacterMovement` (`/Game/_OurStuff/Blueprints/BPM_Actor.GetMyHamster`))))))

(event `Reverse`
  (goto _label :!via `Reverse`))

(fn `UserConstructionScript`
  (`parent.UserConstructionScript`))