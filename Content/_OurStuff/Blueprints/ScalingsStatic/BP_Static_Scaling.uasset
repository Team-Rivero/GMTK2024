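; BP_Static_Scaling is a static mesh object that can shrink or grow, highlighted by a Niagara indicator when the hamster's camera looks toward it.
; Shrink/Grow multiplies the target scale within limits, snapping to 1 when near or crossing it, then a timeline interpolates the root's scale.
; Scaling updates the indicator's radius, and Tick widens the look tolerance with size.
; An Invisible option hides the mesh and disables collision, both toggleable by event.
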(event `self.ReceiveBeginPlay`
  (bind _staticmesh (`self.StaticMesh`))
  (bind _returnvalue_x (`KismetMathLibrary.BreakVector` (`SceneComponent.K2_GetComponentScale` (`self.DefaultSceneRoot`))))
  ;[1 1 1] Begin Play
  (bind _output_get (set `self.NewScale` _returnvalue_x))
  (set `self.CurrentScale` _output_get)
  (`self.UpdateParticleSystem`)
  (if (`self.Invisible`)
    (`KismetArrayLibrary.Array_AddUnique` (`self.Tags`) "Invisible")
    (`PrimitiveComponent.SetMaterial` _staticmesh 0 "/Game/_OurStuff/Materials/M_Emissive.M_Emissive")
    (`PrimitiveComponent.SetCollisionEnabled` _staticmesh "NoCollision")
    (`SceneComponent.SetVisibility` _staticmesh false false)))

(event `self.ReceiveTick`
  (params (DeltaSeconds :type "Float (single-precision)"))
  (bind _ns_scalableindicator (`self.NS_ScalableIndicator`))
  (bind _returnvalue_x (`KismetMathLibrary.BreakVector` (`SceneComponent.K2_GetComponentScale` (`self.DefaultSceneRoot`))))
  (bind _firstpersoncamera (`/Game/_OurStuff/Blueprints/FirstPerson/Blueprints/BP_Hamster.FirstPersonCamera` (`/Game/_OurStuff/Blueprints/BPM_Actor.GetMyHamster`)))
  ;[1 0.3694 0.3097] Tick
  (if (> (`KismetMathLibrary.Dot_VectorVector` (`SceneComponent.GetForwardVector` _firstpersoncamera) (`KismetMathLibrary.Normal` (- (`SceneComponent.K2_GetComponentLocation` (`self.StaticMesh`)) (`SceneComponent.K2_GetComponentLocation` _firstpersoncamera)))) (- 1.0 (* (`self.PlayerLookTolerance`) _returnvalue_x)))
    (`ActorComponent.SetActive` _ns_scalableindicator true false)
    (else
      (`ActorComponent.SetActive` _ns_scalableindicator false false))))

(event `/Game/_OurStuff/Blueprints/BPI_ShrinkGrow.Shrink/Grow`
  (params (`Shrink/Grow Scalar` :type "Float (double-precision)") (`Just Timeline` :type Boolean))
  (bind _newscale (`self.NewScale`))
  (bind _returnvalue_x (`KismetMathLibrary.BreakVector` (`SceneComponent.K2_GetComponentScale` (`self.DefaultSceneRoot`))))
  (bind _returnvalue_x_2 (`KismetMathLibrary.BreakVector` (`SceneComponent.K2_GetComponentScale` (`self.DefaultSceneRoot`))))
  (bind _returnvalue (`KismetMathLibrary.FClamp` (* `Shrink/Grow Scalar` (`self.NewScale`)) (`self.ShrinkLimit`) (`self.GrowthLimit`)))
  (bind _returnvalue_2 (- _returnvalue 1.0))
  ;[1 1 1] Shrink/Grow
  (set `self.CurrentScale` _returnvalue_x_2)
  (if (not `Just Timeline`)
    (if (and (or (== (`KismetMathLibrary.SignOfFloat` (- _newscale 1.0)) (`KismetMathLibrary.SignOfFloat` _returnvalue_2)) (== _newscale 1.0)) (> (`KismetMathLibrary.Abs` _returnvalue_2) (`self.ScaleToOneRange`)))
      (set `self.NewScale` _returnvalue)
      (else
        (set `self.NewScale` 1.0)))
    (set `self.Scaling` true)
    (bind (_direction _alpha) (`Timeline|Scale` :!via `PlayFromStart` :!label _label)
      (:`Update`
        (set `self.Alpha` _alpha)
        (bind _returnvalue_3 (`KismetMathLibrary.Lerp` (`self.CurrentScale`) (`self.NewScale`) _alpha))
        (set `self.ScaleChange` (- _returnvalue_3 _returnvalue_x))
        (`SceneComponent.SetWorldScale3D` (`self.DefaultSceneRoot`) (`KismetMathLibrary.Conv_DoubleToVector` _returnvalue_3))
        (`self.UpdateParticleSystem`))
      (:`Finished`
        (`SceneComponent.SetWorldScale3D` (`self.DefaultSceneRoot`) (`KismetMathLibrary.Conv_DoubleToVector` (`self.NewScale`)))
        (set `self.Scaling` false)
        (`self.UpdateParticleSystem`)))
    (else
      (goto _label :!via `PlayFromStart`))))

(event `/Game/_OurStuff/Blueprints/BPI_Invisible.ToggleCollisionAndVisibility`
  (bind _staticmesh (`self.StaticMesh`))
  ;[1 1 1] Collision and Visibility
  (if (`self.Collision State`)
    (`PrimitiveComponent.SetCollisionEnabled` _staticmesh "NoCollision")
    (else
      (`PrimitiveComponent.SetCollisionEnabled` _staticmesh "QueryAndProbe")))
  (bind _output_get (set `self.Collision State` (not (`self.Collision State`))))
  (`SceneComponent.SetVisibility` (`self.StaticMesh`) _output_get false))

(fn `GetDeltaScale`
  (returns (DeltaScale :type "Float (double-precision)"))
  (return (`self.ScaleChange`)))

(fn `GetScaling`
  (returns (Scaling :type Boolean))
  (return (`self.Scaling`)))

(fn `ReverseScale`
  (locals (TempScale :type "Float (double-precision)"))
  (set `local.TempScale` (`self.NewScale`))
  (set `self.NewScale` 0.0))

(fn `UpdateParticleSystem`
  (bind _returnvalue_x (`KismetMathLibrary.BreakVector` (`SceneComponent.K2_GetComponentScale` (`self.DefaultSceneRoot`))))
  (`NiagaraComponent.SetVariableFloat` (`self.NS_ScalableIndicator`) "BoundingRadius" (* (`.SphereRadius` (`KismetSystemLibrary.GetComponentBounds` (`self.StaticMesh`))) _returnvalue_x)))

(fn `UserConstructionScript`)