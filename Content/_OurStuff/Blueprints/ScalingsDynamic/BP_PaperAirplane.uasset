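; A scalable paper airplane actor that, once its mesh reaches three times scale, flies forward and can carry the player's hamster.
; Tick applies a forward and upward impulse to the dynamic mesh each frame while enlarged.
; A DoOnce adds an initial upward kick, also launching an overlapping hamster, and re-arms when the plane is smaller.
; Box overlap tracks the hamster and zeroes its standing downward force until it leaves.
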(event `ResetInitBoost`
  (goto _label :!via `Reset`))

(event `self.ReceiveTick`
  (params (DeltaSeconds :type "Float (single-precision)"))
  (bind _returnvalue_x (`KismetMathLibrary.BreakVector` (`SceneComponent.K2_GetComponentScale` (`self.DynamicMesh`))))
  (`parent.ReceiveTick` DeltaSeconds)
  (if (>= _returnvalue_x 3.0)
    (`|ExecutionSequence`
      (:`then_0`
        (`/Engine/EditorBlueprintResources/StandardMacros.DoOnce` false :!label _label
          (:`Completed`
            (if (`self.OverlappingCharacter`)
              (`Character.LaunchCharacter` (`/Game/_OurStuff/Blueprints/BPM_Actor.GetMyHamster`) (0.0 0.0 100.0) false false))
            (`PrimitiveComponent.AddImpulse` (`self.DynamicMesh`) (0.0 0.0 100.0) "None" true))))
      (:`then_1`
        (`PrimitiveComponent.AddImpulse` (`self.DynamicMesh`) (+ (* (`self.GetActorForwardVector`) 9.0) (0.0 0.0 6.5)) "None" true)))
    (else
      (`self.ResetInitBoost`))))

(event `self.Box.OnComponentBeginOverlap`
  (params (OverlappedComponent :type "PrimitiveComponent Object Reference") (OtherActor :type "Actor Object Reference") (OtherComp :type "PrimitiveComponent Object Reference") (OtherBodyIndex :type Integer) (bFromSweep :type Boolean) (SweepResult :type "HitResult Structure (by ref)"))
  (set `CharacterMovementComponent.StandingDownwardForceScale` 0.0 (`Character.CharacterMovement` (`/Game/_OurStuff/Blueprints/BPM_Actor.GetMyHamster`)))
  (set `self.OverlappingCharacter` true))

(event `self.Box.OnComponentEndOverlap`
  (params (OverlappedComponent :type "PrimitiveComponent Object Reference") (OtherActor :type "Actor Object Reference") (OtherComp :type "PrimitiveComponent Object Reference") (OtherBodyIndex :type Integer))
  (set `CharacterMovementComponent.StandingDownwardForceScale` 5.0 (`Character.CharacterMovement` (`/Game/_OurStuff/Blueprints/BPM_Actor.GetMyHamster`)))
  (set `self.OverlappingCharacter` false))

(fn `UserConstructionScript`
  (`parent.UserConstructionScript`))