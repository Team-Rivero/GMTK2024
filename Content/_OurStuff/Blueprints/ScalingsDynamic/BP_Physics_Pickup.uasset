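; Physics pickup the hamster player can carry while its scale stays within a carry limit, extending a parent that appears to handle shrinking and growing.
; Tick uses distance and view-direction checks to register it as interactable and show its widget.
; Interact toggles holding, switching gravity and Pawn collision.
; While held, it sweeps to the hamster's hold point every frame, dropping if oversized; dropping zeroes velocities and throttles tick.
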(event `self.ReceiveBeginPlay`
  (`parent.ReceiveBeginPlay`))

(event `self.ReceiveTick`
  (params (DeltaSeconds :type "Float (single-precision)"))
  (bind _asbp_hampster (`/Game/_OurStuff/Blueprints/BPM_Actor.GetMyHamster`))
  (bind _asbp_hampster_2 (`/Game/_OurStuff/Blueprints/BPM_Actor.GetMyHamster`))
  (bind _widget (`self.Widget`))
  (bind _returnvalue_x (`KismetMathLibrary.BreakVector` (`SceneComponent.K2_GetComponentScale` (`self.DynamicMesh`))))
  (bind _returnvalue_x_2 (`KismetMathLibrary.BreakVector` (`SceneComponent.K2_GetComponentScale` (`self.DynamicMesh`))))
  (bind _interactingactors (`/Game/_OurStuff/Blueprints/FirstPerson/Blueprints/BP_Hamster.InteractingActors` _asbp_hampster))
  (bind _returnvalue (`KismetArrayLibrary.Array_Contains` (`/Game/_OurStuff/Blueprints/FirstPerson/Blueprints/BP_Hamster.InteractingActors` _asbp_hampster) self))
  (bind _returnvalue_2 (- (`SceneComponent.K2_GetComponentLocation` (`self.DynamicMesh`)) (`SceneComponent.K2_GetComponentLocation` (`/Game/_OurStuff/Blueprints/FirstPerson/Blueprints/BP_Hamster.FirstPersonCamera` (`/Game/_OurStuff/Blueprints/BPM_Actor.GetMyHamster`)))))
  ;[1 0.276 0.276] Tick
  (`parent.ReceiveTick` DeltaSeconds) ; Shrink/Grow
  (if (`self.Held`)
    (if (<= _returnvalue_x_2 (`self.Max Carry Scale`))
      (`SceneComponent.K2_SetWorldLocationAndRotation` (`self.DynamicMesh`) (`SceneComponent.K2_GetComponentLocation` (`/Game/_OurStuff/Blueprints/FirstPerson/Blueprints/BP_Hamster.Held Object` _asbp_hampster_2)) (`SceneComponent.K2_GetComponentRotation` (`/Game/_OurStuff/Blueprints/FirstPerson/Blueprints/BP_Hamster.Arrow1` _asbp_hampster_2)) true false)
      (`self.SetActorTickInterval` 0.0)
      (else
        (`self.StopHolding`)))
    (elif (and (< (`KismetMathLibrary.VSize` _returnvalue_2) (`self.Pickup Distance`)) (> (`KismetMathLibrary.Dot_VectorVector` (`KismetMathLibrary.Normal` _returnvalue_2) (`KismetMathLibrary.GetForwardVector` (`Pawn.GetControlRotation` (`/Game/_OurStuff/Blueprints/BPM_Actor.GetMyHamster`)))) (- 1.0 (`self.Pickup Tolerance`))))
      (if (and (<= _returnvalue_x (`self.Max Carry Scale`)) (not _returnvalue))
        (`KismetArrayLibrary.Array_AddUnique` _interactingactors self)
        (`SceneComponent.SetHiddenInGame` _widget false false))
      (elif _returnvalue
        (`KismetArrayLibrary.Array_RemoveItem` _interactingactors self)
        (`SceneComponent.SetHiddenInGame` _widget true false)))))

(event `/Game/_OurStuff/Blueprints/BPI_Interact.Interact`
  (bind _asbp_hampster (`/Game/_OurStuff/Blueprints/BPM_Actor.GetMyHamster`))
  (bind _dynamicmesh (`self.DynamicMesh`))
  (bind _dynamicmesh_2 (`self.DynamicMesh`))
  (bind _returnvalue_x (`KismetMathLibrary.BreakVector` (`SceneComponent.K2_GetComponentScale` (`self.DynamicMesh`))))
  (bind _heldobject (`/Game/_OurStuff/Blueprints/FirstPerson/Blueprints/BP_Hamster.HeldObject` (`/Game/_OurStuff/Blueprints/BPM_Actor.GetMyHamster`)))
  ;[1 1 1] Interact
  (if (and _heldobject (`self.Held`))
    (set `/Game/_OurStuff/Blueprints/FirstPerson/Blueprints/BP_Hamster.HeldObjectBuffer` false _asbp_hampster :!label _label) ; Drop
    (set `self.Held` false)
    (`PrimitiveComponent.SetEnableGravity` _dynamicmesh true)
    (`PrimitiveComponent.SetCollisionResponseToChannel` _dynamicmesh_2 "ECC_Pawn" "ECR_Block")
    (`self.SetActorTickInterval` 0.02)
    (`PrimitiveComponent.SetPhysicsLinearVelocity` _dynamicmesh (0.0 0.0 0.0) false "None" :!label _label_2)
    (`PrimitiveComponent.SetPhysicsAngularVelocityInDegrees` _dynamicmesh (0.0 0.0 0.0) false "None")
    (elif (and (not _heldobject) (<= _returnvalue_x (`self.Max Carry Scale`)))
      (set `self.Held` true)
      (set `/Game/_OurStuff/Blueprints/FirstPerson/Blueprints/BP_Hamster.HeldObjectBuffer` true _asbp_hampster)
      (`PrimitiveComponent.SetEnableGravity` _dynamicmesh false)
      (`PrimitiveComponent.SetCollisionResponseToChannel` _dynamicmesh_2 "ECC_Pawn" "ECR_Ignore")
      (goto _label_2))))

(event `StopHolding`
  ;[1 1 1] Interact
  (goto _label))

(fn `UserConstructionScript`)