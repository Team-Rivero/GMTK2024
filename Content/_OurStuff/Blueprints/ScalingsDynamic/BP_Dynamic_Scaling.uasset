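; Physics object that shrinks and grows within limits, with sounds and a Niagara indicator shown when the player hamster looks at it.
; A timeline lerps the scale, snapping to default near or across the original size; Tick applies it, offsetting growth from the last hit pivot.
; Contact with another scaling object applies a push impulse from its scale delta.
; Optional modes hide it until toggled or withhold physics until a scale threshold.
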(event `self.ReceiveBeginPlay`
  (bind _dynamicmesh (`self.DynamicMesh`))
  (bind _returnvalue_x (`KismetMathLibrary.BreakVector` (`SceneComponent.K2_GetComponentScale` (`self.DynamicMesh`))))
  ;[1 1 1] Begin Play
  (`|ExecutionSequence`
    (:`then_0`
      (bind _output_get (set `self.DefaultScale` _returnvalue_x))
      (bind _output_get_2 (set `self.NewScale` _output_get))
      (set `self.SetScale` (`KismetMathLibrary.Conv_DoubleToVector` _output_get_2))
      (`self.UpdateParticleSystem`))
    (:`then_1`
      (if (`self.Invisible`)
        (`KismetArrayLibrary.Array_AddUnique` (`self.Tags`) "Invisible")
        (`PrimitiveComponent.SetMaterial` _dynamicmesh 0 "/Game/_OurStuff/Materials/M_Emissive.M_Emissive")
        (`PrimitiveComponent.SetSimulatePhysics` _dynamicmesh false)
        (`SceneComponent.SetVisibility` _dynamicmesh false false)
        (`PrimitiveComponent.SetCollisionEnabled` _dynamicmesh "NoCollision")
        (if (`self.EnableWeightable`)
          (set `self.DefaultCollision` "QueryAndProbe" :!label _label)
          (set `self.EnablePhysics` false))
        (elif (`self.EnableWeightable`)
          (`PrimitiveComponent.SetSimulatePhysics` _dynamicmesh false)
          (`PrimitiveComponent.SetCollisionEnabled` _dynamicmesh "QueryAndProbe")
          (goto _label))))))

(event `self.ReceiveHit`
  (params (MyComp :type "PrimitiveComponent Object Reference") (Other :type "Actor Object Reference") (OtherComp :type "PrimitiveComponent Object Reference") (bSelfMoved :type Boolean) (HitLocation :type "Vector Structure") (HitNormal :type "Vector Structure") (NormalImpulse :type "Vector Structure") (Hit :type "HitResult Structure (by ref)"))
  ;[1 1 1] accurate pivoting
  (if (`KismetMathLibrary.BooleanNOR` (`GameplayStatics.ObjectIsA` Other "/Game/_OurStuff/Blueprints/FirstPerson/Blueprints/BP_Hamster.BP_Hamster_C") (`GameplayStatics.ObjectIsA` Other "/Game/_OurStuff/Blueprints/FirstPerson/Blueprints/BP_RayProjectile.BP_RayProjectile_C"))
    (set `self.scalePivot` (`KismetMathLibrary.Vector_ProjectOnToNormal` (- HitLocation (`SceneComponent.K2_GetComponentLocation` (`self.DynamicMesh`))) HitNormal))
    (if (`KismetSystemLibrary.DoesImplementInterface` Other "/Game/_OurStuff/Blueprints/BPI_ShrinkGrow.BPI_ShrinkGrow_C")
      (bind _scaling (message `/Game/_OurStuff/Blueprints/BPI_ShrinkGrow.Get Scaling` Other))
      (if (and _scaling (not (`self.Scaling`)))
        (bind _deltascale (message `/Game/_OurStuff/Blueprints/BPI_ShrinkGrow.Get Delta Scale` Other))
        (`PrimitiveComponent.AddVelocityChangeImpulseAtLocation` (`self.DynamicMesh`) (* _deltascale (`KismetMathLibrary.Vector_ProjectOnToNormal` (- HitLocation (`SceneComponent.K2_GetComponentLocation` (`Actor.RootComponent` Other))) HitNormal) (`PrimitiveComponent.GetMass` (`self.DynamicMesh`)) (`self.ScalablePushScalar`)) HitLocation "None")))))

(event `self.ReceiveTick`
  (params (DeltaSeconds :type "Float (single-precision)"))
  (bind _asbp_hampster (`/Game/_OurStuff/Blueprints/BPM_Actor.GetMyHamster`))
  (bind _dynamicmesh (`self.DynamicMesh`))
  (bind _scalepivot (`self.scalePivot`))
  (bind _ns_scalableindicator (`self.NS_ScalableIndicator`))
  (bind _setscale_x (`KismetMathLibrary.BreakVector` (`self.SetScale`)))
  (bind _returnvalue_x (`KismetMathLibrary.BreakVector` (`SceneComponent.K2_GetComponentScale` (`self.DynamicMesh`))))
  (bind _returnvalue_x_2 (`KismetMathLibrary.BreakVector` (`SceneComponent.K2_GetComponentScale` (`self.DynamicMesh`))))
  (bind _returnvalue_x_3 (`KismetMathLibrary.BreakVector` (`SceneComponent.K2_GetComponentScale` (`self.DynamicMesh`))))
  (bind _firstpersoncamera (`/Game/_OurStuff/Blueprints/FirstPerson/Blueprints/BP_Hamster.FirstPersonCamera` _asbp_hampster))
  (bind _returnvalue (- _setscale_x _returnvalue_x_2))
  (bind _returnvalue_2 (* _scalepivot _returnvalue))
  ;[1 1 1] tick
  (`/Engine/EditorBlueprintResources/StandardMacros.IsValid` _asbp_hampster
    (:`Is Valid`
      (if (> (`KismetMathLibrary.Dot_VectorVector` (`SceneComponent.GetForwardVector` _firstpersoncamera) (`KismetMathLibrary.Normal` (- (`SceneComponent.K2_GetComponentLocation` (`self.DynamicMesh`)) (`SceneComponent.K2_GetComponentLocation` _firstpersoncamera)))) (- 1.0 (* (`self.PlayerLookTolerance`) _returnvalue_x_3)))
        (`ActorComponent.SetActive` _ns_scalableindicator true false)
        (else
          (`ActorComponent.SetActive` _ns_scalableindicator false false)))
      (`PrimitiveComponent.WakeAllRigidBodies` (`self.DynamicMesh`))
      (if (and (`self.EnableWeightable`) (>= _returnvalue_x (`self.MaxScaleBeforePhysicsEnabled`)))
        (set `self.EnableWeightable` false)
        (`self.EnableWeightablePhysics` true))
      (if (`self.Scaling`)
        (set `self.DeltaScale` _returnvalue)
        (set `self.scalePivot` (+ _scalepivot _returnvalue_2))
        (`SceneComponent.K2_AddWorldOffset` _dynamicmesh (* _returnvalue_2 (`KismetMathLibrary.SelectFloat` -1.0 0.0 (> (`self.NewScale`) (`self.CurrentScale`)))) false false)
        (`SceneComponent.SetWorldScale3D` _dynamicmesh (`self.SetScale`))
        (`self.UpdateParticleSystem`)))))

(event `/Game/_OurStuff/Blueprints/BPI_ShrinkGrow.Shrink/Grow`
  (params (`Shrink/Grow Scalar` :type "Float (double-precision)") (`Just Timeline` :type Boolean) (`Grow/Shrink` :type Boolean))
  (bind _newscale (`self.NewScale`))
  (bind _defaultscale (`self.DefaultScale`))
  (bind _returnvalue_x (`KismetMathLibrary.BreakVector` (`SceneComponent.K2_GetComponentScale` (`self.DynamicMesh`))))
  (bind _returnvalue (`KismetMathLibrary.FClamp` (* `Shrink/Grow Scalar` (`self.NewScale`)) (`self.ShrinkLimit`) (`self.GrowthLimit`)))
  (bind _returnvalue_2 (- _returnvalue _defaultscale))
  ;[1 1 1] shrink/grow
  (set `self.CurrentScale` _returnvalue_x)
  (`|ExecutionSequence`
    (:`then_0`
      (`self.Audio` `Grow/Shrink`))
    (:`then_1`
      (if (and (or (== (`KismetMathLibrary.SignOfFloat` (- _newscale _defaultscale)) (`KismetMathLibrary.SignOfFloat` _returnvalue_2)) (== _newscale _defaultscale)) (> (`KismetMathLibrary.Abs` _returnvalue_2) (`self.ScaleToDefaultRange`)))
        (set `self.NewScale` _returnvalue)
        (bind (_direction _alpha) (`Timeline|Timeline` :!via `PlayFromStart` :!label _label_2)
          (:`Update`
            (set `self.Scaling` true)
            (set `self.SetScale` (`KismetMathLibrary.Conv_DoubleToVector` (`KismetMathLibrary.Lerp` (`self.CurrentScale`) (`self.NewScale`) _alpha))))
          (:`Finished`
            (`SceneComponent.SetWorldScale3D` (`self.DynamicMesh`) (`KismetMathLibrary.Conv_DoubleToVector` (`self.NewScale`)))
            (set `self.Scaling` false)))
        (else
          (set `self.NewScale` (`self.DefaultScale`))
          (goto _label_2 :!via `PlayFromStart`))))))

(event `/Game/_OurStuff/Blueprints/BPI_Invisible.ToggleCollisionAndVisibility`
  (bind _dynamicmesh (`self.DynamicMesh`))
  (bind _dynamicmesh_2 (`self.DynamicMesh`))
  ;[1 1 1] Collision and Visibility
  (if (`self.Invisible`)
    (bind _output_get (set `self.CollisionState` (not (`self.CollisionState`))))
    (`SceneComponent.SetVisibility` _dynamicmesh _output_get false)
    (`PrimitiveComponent.SetSimulatePhysics` _dynamicmesh (and _output_get (`self.EnablePhysics`)))
    (if _output_get
      (`PrimitiveComponent.SetCollisionEnabled` _dynamicmesh_2 (`self.DefaultCollision`))
      (else
        (`PrimitiveComponent.SetCollisionEnabled` _dynamicmesh_2 "NoCollision")))))

(event `/Game/_OurStuff/Blueprints/BPI_Weighable.EnableWeightablePhysics`
  (params (bool :type Boolean))
  (bind _dynamicmesh (`self.DynamicMesh`))
  ;[1 1 1] Enable/Disable Weightable Physics
  (bind _output_get (set `self.EnablePhysics` bool))
  (if _output_get
    (set `self.DefaultCollision` "QueryAndPhysics")
    (else
      (set `self.DefaultCollision` "QueryAndProbe")))
  (if (`KismetMathLibrary.BooleanNAND` (`self.Invisible`) (not (`self.CollisionState`)))
    (`PrimitiveComponent.SetSimulatePhysics` _dynamicmesh (`self.EnablePhysics`))
    (`PrimitiveComponent.SetCollisionEnabled` _dynamicmesh (`self.DefaultCollision`))))

(fn `Audio`
  (params (`Grow/Shrink` :type Boolean))
  (bind _currentscale (`self.CurrentScale`))
  (if `Grow/Shrink`
    (if (not (`KismetMathLibrary.NearlyEqual_FloatFloat` (`self.GrowthLimit`) _currentscale))
      (`GameplayStatics.PlaySound2D` "/Game/_OurStuff/Audio/Grow.Grow" 0.5 (`KismetMathLibrary.RandomFloatInRange` 0.8 1.2) 0.0 null null))
    (elif (not (`KismetMathLibrary.NearlyEqual_FloatFloat` _currentscale (`self.ShrinkLimit`)))
      (`GameplayStatics.PlaySound2D` "/Game/_OurStuff/Audio/Shrink.Shrink" 0.5 (`KismetMathLibrary.RandomFloatInRange` 0.8 1.2) 0.0 null null))))

(fn `Get Delta Scale`
  (returns (DeltaScale :type "Float (double-precision)"))
  (return (`self.DeltaScale`)))

(fn `Get Scaling`
  (returns (Scaling :type Boolean))
  (return (`self.Scaling`)))

(fn `UpdateParticleSystem`
  (`NiagaraComponent.SetVariableFloat` (`self.NS_ScalableIndicator`) "BoundingRadius" (`.SphereRadius` (`KismetSystemLibrary.GetComponentBounds` (`self.DynamicMesh`)))))

(fn `UserConstructionScript`)